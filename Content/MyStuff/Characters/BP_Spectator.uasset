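; BP_Spectator is a spectator pawn that lets a player respawn into PvP play by pressing R.
; The key press async-loads the PVP_SaveGame from the save slot and passes the saved appearance and weapon type to a server respawn event.
; That event spawns a BP_PVP_Player at the spectator's transform with those settings, owned by the controller, which then possesses it.
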(event Custom|Server_Respawn
  (params (Appearance_Settings :type S%20Yoll%20Appearance%20Settings%20Structure) (WeaponType :type EWeaponTypes%20Enum :default "Katana"))
  (bind _returnvalue (Game|SpawnActorfromClass "/Game/MyStuff/Characters/BP_PVP_Player.BP_PVP_Player_C" (Transformation|GetActorTransform) "AdjustIfPossibleButAlwaysSpawn" "MultiplyWithRoot" (Pawn|GetController) Appearance_Settings WeaponType 0))
  (Pawn|Possess (Pawn|GetController) _returnvalue))

(event EventBeginPlay)

(event Collision|EventActorBeginOverlap
  (params (OtherActor :type Actor%20Object%20Reference)))

(event EventTick
  (params (DeltaSeconds :type Float%20%28single-precision%29)))

(event Input|KeyboardEvents|R
  (params (Key :type Key%20Structure :default "None"))
  (:Pressed
    (bind _savegame (|AsyncLoadGamefromSlot "SaveSlot")
      (:Completed
        (bind _aspvp_save_game (Utilities|Casting|CastToPVP_SaveGame _savegame))
        (CallFunction|ServerRespawn (Variables|/Game/MyStuff/Systems/PVP_SaveGame.PVP_SaveGame_C|GetPlayerAppearance _aspvp_save_game) (Variables|/Game/MyStuff/Systems/PVP_SaveGame.PVP_SaveGame_C|GetWeaponType _aspvp_save_game))))))

(fn ConstructionScript)