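; BP_PVP_Player is a player character Blueprint with automatic blinking and mouse-wheel camera zoom.
; On BeginPlay, a timeline drives two Japanese-named wink morph targets on the Mesh, replaying after a random delay of a few seconds.
; The wheel adjusts the CameraBoom arm length by a scaled rate within clamped limits.
; The construction script makes the Outline component follow the Mesh through leader pose.
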(event EventBeginPlay
  (|CallParentFunction)
  (bind _alpha (Timeline|Blink_Timeline PlayFromStart)
    (:Update
      (Components|SkeletalMesh|SetMorphTarget (Variables|Character|GetMesh) "ウィンク２" _alpha true)
      (Components|SkeletalMesh|SetMorphTarget (Variables|Character|GetMesh) "ｳｨﾝｸ２右" _alpha true))
    (:Finished
      (Utilities|FlowControl|Delay (Math|Random|RandomFloatinRange 4.0 6.0))
      (Timeline|Blink_Timeline PlayFromStart))))

(event Collision|EventActorBeginOverlap
  (params (OtherActor :type Actor%20Object%20Reference)))

(event EventTick
  (params (DeltaSeconds :type Float%20%28single-precision%29)))

(event Input|MouseEvents|MouseWheelUp
  (params (Key :type Key%20Structure))
  (bind _cameraboom (Variables|Default|GetCameraBoom))
  (:Pressed
    (Variables|/Script/Engine.SpringArmComponent|SetTargetArmLength _cameraboom (Math|Float|Clamp(Float) (- (Variables|/Script/Engine.SpringArmComponent|GetTargetArmLength _cameraboom) (* (Variables|Default|GetCameraScaleRate) 1e+01)) 5e+01 4.5e+02))))

(event Input|MouseEvents|MouseWheelDown
  (params (Key :type Key%20Structure))
  (bind _cameraboom (Variables|Default|GetCameraBoom))
  (:Pressed
    (Variables|/Script/Engine.SpringArmComponent|SetTargetArmLength _cameraboom (Math|Float|Clamp(Float) (+ (Variables|/Script/Engine.SpringArmComponent|GetTargetArmLength _cameraboom) (* (Variables|Default|GetCameraScaleRate) 1e+01)) 5e+01 4.5e+02))))

(fn ConstructionScript
  (Components|SkinnedMesh|SetLeaderPoseComponent (Variables|Default|GetOutline) (Variables|Character|GetMesh) true false))