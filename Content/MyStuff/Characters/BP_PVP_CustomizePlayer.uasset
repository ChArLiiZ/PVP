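; Customizable player character for PVP customization that builds its look from AppearanceSettings and displays a selected weapon.
; UpdateAppearance, run on construction and BeginPlay, assembles leader-posed hair, tail, clothing and horn meshes, applying morph targets, dynamic MToon materials, and skin and eye textures.
; Most parts get toon outlines from negatively scaled duplicate meshes.
; ChangeWeaponType async-loads and spawns the weapon, attaches it by socket and swaps the animation Blueprint.
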(event Custom|Change%20Weapon%20Type
  (params (WeaponType :type EWeaponTypes%20Enum :default "Katana"))
  (Variables|Default|SetWeaponType WeaponType)
  (if (.ReturnValue (Utilities|Map|Find (Variables|Default|GetWeaponBPs) (Variables|Default|GetWeaponType)))
    (bind _class (Utilities|AsyncLoadClassAsset (.Value (Utilities|Map|Find (Variables|Default|GetWeaponBPs) (Variables|Default|GetWeaponType))))
      (:Completed
        (bind _asbp_weapon_base (Utilities|Casting|CastToBP_WeaponBaseClass _class))
        (bind _returnvalue (Game|SpawnActorfromClass _asbp_weapon_base (Transformation|GetActorTransform) "AlwaysSpawn" "MultiplyWithRoot" 0 0 0))
        (Default|StopCheck _returnvalue)
        (bind _weaponref (Variables|Default|GetWeaponRef)
          (:then
            (Actor|DestroyActor _weaponref))
          (:else
            _))
        (Variables|Default|SetWeaponRef _returnvalue)
        (Transformation|AttachComponentToComponent (Variables|/Script/PVP.WeaponBase|GetSKMesh _returnvalue) (Variables|Default|GetMesh) (.SocketName (Utilities|Struct|BreakWeaponAttributes (Variables|/Script/PVP.WeaponInfos|GetAttributes (.Value (Utilities|Map|Find (Variables|Default|GetWeaponInfos) (Variables|Default|GetWeaponType)))))) "SnapToTarget" "SnapToTarget" "KeepWorld" true)
        (Class|SkeletalMeshComponent|SetAnimClass (Variables|Default|GetMesh) (.AnimBP (Utilities|Struct|BreakWeaponAnimations (Variables|/Script/PVP.WeaponInfos|GetAnimations (.Value (Utilities|Map|Find (Variables|Default|GetWeaponInfos) (Variables|Default|GetWeaponType)))))))
        (Class|WeaponBase|AdditionalSetup (Variables|Default|GetWeaponRef) (Variables|Default|GetMesh))))))

(event EventBeginPlay
  (|CallParentFunction)
  (CallFunction|UpdateAppearance)
  (CallFunction|ChangeWeaponType (Variables|Default|GetWeaponType)))

(event EventTick
  (params (DeltaSeconds :type Float%20%28single-precision%29))
  (|CallParentFunction DeltaSeconds))

(fn ConstructionScript
  (Components|SkinnedMesh|SetLeaderPoseComponent (Variables|Default|GetOutline) (Variables|Default|GetMesh) true true)
  (CallFunction|UpdateAppearance))

(fn SetHair
  (bind _appearance_settings (Variables|Appearance|GetAppearance_Settings))
  (bind _appearance_settings_2 (Variables|Appearance|GetAppearance_Settings))
  (bind _returnvalue (select (.twintail _appearance_settings) 0 "/Game/MyStuff/Characters/Yoll/Meshes/Hairs/Yoll_OriginalHair.Yoll_OriginalHair"))
  ;[1 0 0.7969] Hair
  (Utilities|IsValid (Variables|Appearance|GetHairRef)
    (:Is%20Valid
      _)
    (:Is%20Not%20Valid
      (bind _returnvalue_2 (AddComponent|AddSkeletalMeshComponent false))
      (Variables|Appearance|SetHairRef _returnvalue_2)))
  (Components|SkinnedMesh|SetLeaderPoseComponent (Variables|Appearance|GetHairRef) (Variables|Default|GetMesh) false false)
  (Transformation|AttachComponentToComponent (Variables|Appearance|GetHairRef) (Variables|Default|GetMesh) "None" "SnapToTarget" "SnapToTarget" "SnapToTarget" true)
  (Components|SkeletalMesh|SetSkeletalMeshAsset (Variables|Appearance|GetHairRef) _returnvalue)
  (bind _returnvalue_3 (Rendering|Material|CreateDynamicMaterialInstance (Variables|Appearance|GetHairRef) 0 (Rendering|Material|GetMaterial (Variables|Appearance|GetHairRef) 0) "None" :!class /Script/Engine.PrimitiveComponent))
  (Rendering|Material|SetVectorParameterValue _returnvalue_3 "mtoon_Color" (.haircolor _appearance_settings_2) :!class /Script/Engine.MaterialInstanceDynamic)
  (Rendering|Material|SetVectorParameterValue _returnvalue_3 "mtoon_ShadeColor" (* (.haircolor _appearance_settings_2) "(R=0.700000,G=0.700000,B=0.700000,A=1.000000)") :!class /Script/Engine.MaterialInstanceDynamic)
  (Rendering|Material|SetMaterial (Variables|Appearance|GetHairRef) 0 _returnvalue_3)
  (Utilities|IsValid (Variables|Appearance|GetHair_Outline_Ref)
    (:Is%20Valid
      _)
    (:Is%20Not%20Valid
      (bind _returnvalue_4 (AddComponent|AddSkeletalMeshComponent false (Math|Transform|MakeTransform "0, 0, 0" "0, 0, 0" "-1.000000,-1.000000,-1.000000")))
      (Variables|Appearance|SetHair_Outline_Ref _returnvalue_4)))
  (Rendering|SetBoundsScale (Variables|Appearance|GetHair_Outline_Ref) 5.0)
  (Components|SkeletalMesh|SetSkeletalMeshAsset (Variables|Appearance|GetHair_Outline_Ref) _returnvalue)
  (Rendering|Material|SetMaterial (Variables|Appearance|GetHair_Outline_Ref) 0 "/Game/MyStuff/Characters/Yoll/Meshes/Materials/M_Yoll_Hair_Outline.M_Yoll_Hair_Outline")
  (Rendering|Material|SetMaterial (Variables|Appearance|GetHair_Outline_Ref) 1 "/Game/MyStuff/Characters/Yoll/Meshes/Materials/M_Yoll_Hair_Outline.M_Yoll_Hair_Outline")
  (Components|SkinnedMesh|SetLeaderPoseComponent (Variables|Appearance|GetHair_Outline_Ref) (Variables|Appearance|GetHairRef) false false)
  (Transformation|AttachComponentToComponent (Variables|Appearance|GetHair_Outline_Ref) (Variables|Default|GetMesh) "None" "SnapToTarget" "SnapToTarget" "KeepWorld" true)
  ;[0 1 0.5781] Tail
  (Utilities|IsValid (Variables|Appearance|GetTailRef)
    (:Is%20Valid
      _)
    (:Is%20Not%20Valid
      (bind _returnvalue_5 (AddComponent|AddSkeletalMeshComponent false))
      (Variables|Appearance|SetTailRef _returnvalue_5)))
  (Components|SkinnedMesh|SetLeaderPoseComponent (Variables|Appearance|GetTailRef) (Variables|Default|GetMesh) false false)
  (Transformation|AttachComponentToComponent (Variables|Appearance|GetTailRef) (Variables|Default|GetMesh) "None" "SnapToTarget" "SnapToTarget" "SnapToTarget" true)
  (Components|SkeletalMesh|SetSkeletalMeshAsset (Variables|Appearance|GetTailRef) "/Game/MyStuff/Characters/Yoll/Meshes/Outfits/Yoll_Tail.Yoll_Tail")
  (Rendering|Material|SetMaterial (Variables|Appearance|GetTailRef) 0 _returnvalue_3)
  (Utilities|IsValid (Variables|Appearance|GetTail_Outline_Ref)
    (:Is%20Valid
      _)
    (:Is%20Not%20Valid
      (bind _returnvalue_6 (AddComponent|AddSkeletalMeshComponent false (Math|Transform|MakeTransform "0, 0, 0" "0, 0, 0" "-1.000000,-1.000000,-1.000000")))
      (Variables|Appearance|SetTail_Outline_Ref _returnvalue_6)))
  (Rendering|SetBoundsScale (Variables|Appearance|GetTail_Outline_Ref) 1e+01)
  (Components|SkeletalMesh|SetSkeletalMeshAsset (Variables|Appearance|GetTail_Outline_Ref) "/Game/MyStuff/Characters/Yoll/Meshes/Outfits/Yoll_Tail.Yoll_Tail")
  (Rendering|Material|SetMaterial (Variables|Appearance|GetTail_Outline_Ref) 0 "/Game/MyStuff/Characters/Yoll/Meshes/Materials/M_Yoll_Hair_Outline.M_Yoll_Hair_Outline")
  (Components|SkinnedMesh|SetLeaderPoseComponent (Variables|Appearance|GetTail_Outline_Ref) (Variables|Appearance|GetTailRef) false false)
  (Transformation|AttachComponentToComponent (Variables|Appearance|GetTail_Outline_Ref) (Variables|Appearance|GetTailRef) "None" "SnapToTarget" "SnapToTarget" "KeepWorld" true))

(fn SetCloth
  (bind _appearance_settings (Variables|Appearance|GetAppearance_Settings))
  (bind _mune1 (Variables|Appearance|GetMune1))
  (bind _mune2 (Variables|Appearance|GetMune2))
  (bind _appearance_settings_2 (Variables|Appearance|GetAppearance_Settings))
  (bind _appearance_settings_3 (Variables|Appearance|GetAppearance_Settings))
  (bind _tshirt_color (Utilities|Struct|BreakS_Yoll_Appearance_Settings _appearance_settings))
  (bind _flowcat_hood_ (Utilities|Struct|BreakS_Yoll_Appearance_Settings _appearance_settings_2))
  (bind (_skin _eye _twintail _haircolor _horn_ _horn_color _cloth _coat_sleevelength _coat_havepant_ _tshirt_type _tshirt_color_2 _flowcat_type) (Utilities|Struct|BreakS_Yoll_Appearance_Settings _appearance_settings_3))
  (bind _returnvalue (Math|Float|SelectFloat 0.0 1.0 _flowcat_hood_))
  (bind _returnvalue_2 (Utilities|Select :Index _flowcat_type :NewEnumerator0 "/Game/MyStuff/Characters/Yoll/Meshes/Outfits/FlowCat/Textures/t1.t1" :NewEnumerator1 "/Game/MyStuff/Characters/Yoll/Meshes/Outfits/FlowCat/Textures/t2.t2" :NewEnumerator2 "/Game/MyStuff/Characters/Yoll/Meshes/Outfits/FlowCat/Textures/t3.t3" :NewEnumerator3 "/Game/MyStuff/Characters/Yoll/Meshes/Outfits/FlowCat/Textures/t4.t4" :NewEnumerator4 "/Game/MyStuff/Characters/Yoll/Meshes/Outfits/FlowCat/Textures/t5.t5" :NewEnumerator5 "/Game/MyStuff/Characters/Yoll/Meshes/Outfits/FlowCat/Textures/t6.t6" :NewEnumerator6 "/Game/MyStuff/Characters/Yoll/Meshes/Outfits/FlowCat/Textures/t7.t7" :NewEnumerator7 "/Game/MyStuff/Characters/Yoll/Meshes/Outfits/FlowCat/Textures/t8.t8" :NewEnumerator8 "/Game/MyStuff/Characters/Yoll/Meshes/Outfits/FlowCat/Textures/t9.t9" :NewEnumerator9 "/Game/MyStuff/Characters/Yoll/Meshes/Outfits/FlowCat/Textures/t10.t10"))
  (bind _returnvalue_3 (Utilities|Select :Index _tshirt_type :NewEnumerator0 "/Game/MyStuff/Characters/Yoll/Meshes/Outfits/Tshirt/Textures/1.1" :NewEnumerator1 "/Game/MyStuff/Characters/Yoll/Meshes/Outfits/Tshirt/Textures/2.2" :NewEnumerator2 "/Game/MyStuff/Characters/Yoll/Meshes/Outfits/Tshirt/Textures/3.3" :NewEnumerator3 "/Game/MyStuff/Characters/Yoll/Meshes/Outfits/Tshirt/Textures/4.4" :NewEnumerator4 "/Game/MyStuff/Characters/Yoll/Meshes/Outfits/Tshirt/Textures/5.5" :NewEnumerator5 "/Game/MyStuff/Characters/Yoll/Meshes/Outfits/Tshirt/Textures/6.6" :NewEnumerator6 "/Game/MyStuff/Characters/Yoll/Meshes/Outfits/Tshirt/Textures/7.7" :NewEnumerator7 "/Game/MyStuff/Characters/Yoll/Meshes/Outfits/Tshirt/Textures/8.8" :NewEnumerator8 "/Game/MyStuff/Characters/Yoll/Meshes/Outfits/Tshirt/Textures/9.9" :NewEnumerator9 "/Game/MyStuff/Characters/Yoll/Meshes/Outfits/Tshirt/Textures/10.10" :NewEnumerator10 "/Game/MyStuff/Characters/Yoll/Meshes/Outfits/Tshirt/Textures/11.11" :NewEnumerator11 "/Game/MyStuff/Characters/Yoll/Meshes/Outfits/Tshirt/Textures/12.12" :NewEnumerator12 "/Game/MyStuff/Characters/Yoll/Meshes/Outfits/Tshirt/Textures/13.13"))
  (LocalVariables|SetCloth_Mesh (Utilities|Select :Index (.Cloth (Utilities|Struct|BreakS_Yoll_Appearance_Settings (Variables|Appearance|GetAppearance_Settings))) :NewEnumerator0 "/Game/MyStuff/Characters/Yoll/Meshes/Outfits/Coat/DefaultCoat.DefaultCoat" :NewEnumerator2 "/Game/MyStuff/Characters/Yoll/Meshes/Outfits/Tshirt/Tshirt.Tshirt" :NewEnumerator3 "/Game/MyStuff/Characters/Yoll/Meshes/Outfits/FlowCat/FlowCat.FlowCat"))
  (Utilities|IsValid (Variables|Appearance|GetClothRef)
    (:Is%20Valid
      _)
    (:Is%20Not%20Valid
      (bind _returnvalue_4 (AddComponent|AddSkeletalMeshComponent false))
      (Variables|Appearance|SetClothRef _returnvalue_4)))
  (Components|SkinnedMesh|SetLeaderPoseComponent (Variables|Appearance|GetClothRef) (Variables|Default|GetMesh) false false)
  (Transformation|AttachComponentToComponent (Variables|Appearance|GetClothRef) (Variables|Default|GetMesh) "None" "SnapToTarget" "SnapToTarget" "SnapToTarget" true)
  (Components|SkeletalMesh|SetSkeletalMeshAsset (Variables|Appearance|GetClothRef) (LocalVariables|GetCloth_Mesh))
  (CallFunction|ResetClothMaterial)
  (Utilities|IsValid (Variables|Appearance|GetCloth_Outline_Ref)
    (:Is%20Valid
      _)
    (:Is%20Not%20Valid
      (bind _returnvalue_5 (AddComponent|AddSkeletalMeshComponent false (Math|Transform|MakeTransform "0, 0, 0" "0, 0, 0" "-1.000000,-1.000000,-1.000000")))
      (Variables|Appearance|SetCloth_Outline_Ref _returnvalue_5)))
  (Rendering|SetBoundsScale (Variables|Appearance|GetCloth_Outline_Ref) 1e+01)
  (Components|SkinnedMesh|SetLeaderPoseComponent (Variables|Appearance|GetCloth_Outline_Ref) (Variables|Appearance|GetClothRef) true false)
  (Transformation|AttachComponentToComponent (Variables|Appearance|GetCloth_Outline_Ref) (Variables|Default|GetMesh) "None" "SnapToTarget" "SnapToTarget" "KeepWorld" true)
  (Components|SkeletalMesh|SetSkeletalMeshAsset (Variables|Appearance|GetCloth_Outline_Ref) (LocalVariables|GetCloth_Mesh))
  (Utilities|FlowControl|Sequence
    (:then_0
      (for (_array_element _array_index) (Class|MeshComponent|GetMaterialSlotNames (Variables|Appearance|GetCloth_Outline_Ref))
        (Rendering|Material|SetMaterialbyName (Variables|Appearance|GetCloth_Outline_Ref) _array_element (Utilities|Array|Get(acopy) (Utilities|Select :Index (.Cloth (Utilities|Struct|BreakS_Yoll_Appearance_Settings (Variables|Appearance|GetAppearance_Settings))) :NewEnumerator0 (Utilities|Array|MakeArray "/Game/MyStuff/Characters/Yoll/Meshes/Materials/M_Yoll_Crt_Outline.M_Yoll_Crt_Outline" "/Game/MyStuff/Characters/Yoll/Meshes/Outfits/Coat/M_Yoll_Coat_Outline.M_Yoll_Coat_Outline" "/Game/MyStuff/Characters/Yoll/Meshes/Outfits/Coat/M_Yoll_Coat_Outline.M_Yoll_Coat_Outline" "/Game/MyStuff/Characters/Yoll/Meshes/Materials/M_Yoll_Crt_Outline.M_Yoll_Crt_Outline" "/Game/MyStuff/Characters/Yoll/Meshes/Materials/M_Yoll_Crt_Outline.M_Yoll_Crt_Outline" "/Game/MyStuff/Characters/Yoll/Meshes/Materials/M_Yoll_Crt_Outline.M_Yoll_Crt_Outline" "/Game/MyStuff/Characters/Yoll/Meshes/Materials/M_Yoll_Crt_Outline.M_Yoll_Crt_Outline") :NewEnumerator2 (Utilities|Array|MakeArray "/Game/MyStuff/Characters/Yoll/Meshes/Outfits/Tshirt/M_Yoll_Tshirt_Outline.M_Yoll_Tshirt_Outline") :NewEnumerator3 (Utilities|Array|MakeArray "/Game/MyStuff/Characters/Yoll/Meshes/Outfits/FlowCat/M_Yoll_FlowCat_Outline.M_Yoll_FlowCat_Outline" "/Game/MyStuff/Characters/Yoll/Meshes/Outfits/FlowCat/M_Yoll_FlowCat_Outline.M_Yoll_FlowCat_Outline" "/Game/MyStuff/Characters/Yoll/Meshes/Outfits/FlowCat/M_Yoll_FlowCat_Outline.M_Yoll_FlowCat_Outline")) _array_index)))
      (if (not (.coat_havepant? (Variables|Appearance|GetAppearance_Settings)))
        (Rendering|Material|SetMaterialbyName (Variables|Appearance|GetCloth_Outline_Ref) "pant_crt" "/Game/MyStuff/Materials/M_Translucent.M_Translucent")))
    (:then_1
      (switch Utilities|FlowControl|Switch|SwitchonE_Yoll_Cloth_Options _cloth
        (:NewEnumerator0
          (Components|SkeletalMesh|SetMorphTarget (Variables|Appearance|GetClothRef) "Key 4" (.coat_sleevelength (Variables|Appearance|GetAppearance_Settings)) true)
          (Transformation|SetRelativeLocation (Variables|Default|GetMesh) "0.000000,0.000000,-75.655000" false false))
        (:NewEnumerator2
          (Components|SkeletalMesh|SetMorphTarget (Variables|Appearance|GetClothRef) "mune1" (Variables|Appearance|GetMune1) true)
          (Components|SkeletalMesh|SetMorphTarget (Variables|Appearance|GetClothRef) "mune2" (Variables|Appearance|GetMune2) true)
          (Components|SkeletalMesh|SetMorphTarget (Variables|Appearance|GetClothRef) "suso" -1.0 true)
          (Components|SkeletalMesh|SetMorphTarget (Variables|Appearance|GetClothRef) "tyt" 1.0 true)
          (Utilities|IsValid (Variables|Appearance|GetTshirt_DM)
            (:Is%20Valid
              _)
            (:Is%20Not%20Valid
              (bind _returnvalue_6 (Rendering|Material|CreateDynamicMaterialInstance (Variables|Appearance|GetClothRef) 0 (Rendering|Material|GetMaterial (Variables|Appearance|GetClothRef) 0) "None" :!class /Script/Engine.PrimitiveComponent))
              (Variables|Appearance|SetTshirt_DM _returnvalue_6)))
          (Rendering|Material|SetTextureParameterValue (Variables|Appearance|GetTshirt_DM) "gltf_tex_diffuse" _returnvalue_3)
          (Rendering|Material|SetTextureParameterValue (Variables|Appearance|GetTshirt_DM) "mtoon_tex_ShadeTexture" _returnvalue_3)
          (Rendering|Material|SetVectorParameterValue (Variables|Appearance|GetTshirt_DM) "mtoon_Color" _tshirt_color :!class /Script/Engine.MaterialInstanceDynamic)
          (Rendering|Material|SetVectorParameterValue (Variables|Appearance|GetTshirt_DM) "mtoon_ShadeColor" (* _tshirt_color "(R=0.700000,G=0.700000,B=0.700000,A=1.000000)") :!class /Script/Engine.MaterialInstanceDynamic)
          (Rendering|Material|SetMaterial (Variables|Appearance|GetClothRef) 0 (Variables|Appearance|GetTshirt_DM))
          (InitialSetups|SetPantie))
        (:NewEnumerator3
          (Components|SkeletalMesh|SetMorphTarget (Variables|Appearance|GetClothRef) "mune1" _mune1 true)
          (Components|SkeletalMesh|SetMorphTarget (Variables|Appearance|GetClothRef) "mune2" _mune2 true)
          (Components|SkeletalMesh|SetMorphTarget (Variables|Appearance|GetClothRef) "Key 1" _mune1 true)
          (Components|SkeletalMesh|SetMorphTarget (Variables|Appearance|GetClothRef) "Key 2" _mune2 true)
          (Components|SkeletalMesh|SetMorphTarget (Variables|Appearance|GetClothRef) "hide_hood2" _returnvalue true)
          (Components|SkeletalMesh|SetMorphTarget (Variables|Appearance|GetClothRef) "hide_hood1" _returnvalue true)
          (Components|SkeletalMesh|SetMorphTarget (Variables|Appearance|GetClothRef) "hone" (Math|Float|SelectFloat 1.0 0.0 (.Horn? (Utilities|Struct|BreakS_Yoll_Appearance_Settings (Variables|Appearance|GetAppearance_Settings)))) true)
          (Components|SkeletalMesh|SetMorphTarget (Variables|Appearance|GetClothRef) "tale" 1.0 true)
          (Components|SkeletalMesh|SetMorphTarget (Variables|Appearance|GetClothRef) "suso" 0.0 true)
          (Utilities|IsValid (Variables|Appearance|GetFlowCat_DM)
            (:Is%20Valid
              _)
            (:Is%20Not%20Valid
              (bind _returnvalue_7 (Rendering|Material|CreateDynamicMaterialInstance (Variables|Appearance|GetClothRef) 0 (Rendering|Material|GetMaterial (Variables|Appearance|GetClothRef) 0) "None" :!class /Script/Engine.PrimitiveComponent))
              (Variables|Appearance|SetFlowCat_DM _returnvalue_7)))
          (Rendering|Material|SetTextureParameterValue (Variables|Appearance|GetFlowCat_DM) "gltf_tex_diffuse" _returnvalue_2)
          (Rendering|Material|SetTextureParameterValue (Variables|Appearance|GetFlowCat_DM) "mtoon_tex_ShadeTexture" _returnvalue_2)
          (for (_ _array_index_2) (Rendering|Material|GetMaterials (Variables|Appearance|GetClothRef))
            (Rendering|Material|SetMaterial (Variables|Appearance|GetClothRef) _array_index_2 (Variables|Appearance|GetFlowCat_DM))))))
    (:then_2
      (if (Utilities|Enum|Equal(Enum) (.Cloth (Utilities|Struct|BreakS_Yoll_Appearance_Settings (Variables|Appearance|GetAppearance_Settings))) "NewEnumerator0")
        (Transformation|SetRelativeLocation (Variables|Default|GetMesh) "0.000000,0.000000,-79.000000" false false)
        (else
          (Transformation|SetRelativeLocation (Variables|Default|GetMesh) "0.000000,0.000000,-81.000000" false false))))))

(fn SetSkin
  (bind _appearance_settings (Variables|Appearance|GetAppearance_Settings))
  (bind _returnvalue (Utilities|Select :Index (.skin _appearance_settings) :NewEnumerator0 "/Game/MyStuff/Characters/Yoll/Meshes/Textures/tex4_2.tex4_2" :NewEnumerator1 "/Game/MyStuff/Characters/Yoll/Meshes/Textures/tex4_3.tex4_3" :NewEnumerator2 "/Game/MyStuff/Characters/Yoll/Meshes/Textures/tex4_4.tex4_4"))
  (for _array_element (Utilities|Array|MakeArray 0 3)
    (bind _returnvalue_2 (Rendering|Material|CreateDynamicMaterialInstance (Variables|Default|GetMesh) _array_element (Rendering|Material|GetMaterial (Variables|Default|GetMesh) _array_element) "None" :!class /Script/Engine.PrimitiveComponent))
    (Rendering|Material|SetTextureParameterValue _returnvalue_2 "gltf_tex_diffuse" _returnvalue)
    (Rendering|Material|SetTextureParameterValue _returnvalue_2 "mtoon_tex_ShadeTexture" _returnvalue)))

(fn SetEye
  (bind _appearance_settings (Variables|Appearance|GetAppearance_Settings))
  (bind _eye (Utilities|Struct|BreakS_Yoll_Appearance_Settings _appearance_settings))
  (bind _returnvalue (Utilities|Select :Index _eye :NewEnumerator0 "/Game/MyStuff/Characters/Yoll/Meshes/Textures/tex6_1.tex6_1" :NewEnumerator1 "/Game/MyStuff/Characters/Yoll/Meshes/Textures/tex6_2.tex6_2" :NewEnumerator2 "/Game/MyStuff/Characters/Yoll/Meshes/Textures/tex6_3.tex6_3" :NewEnumerator3 "/Game/MyStuff/Characters/Yoll/Meshes/Textures/tex6_4.tex6_4" :NewEnumerator4 "/Game/MyStuff/Characters/Yoll/Meshes/Textures/tex6_5.tex6_5" :NewEnumerator5 "/Game/MyStuff/Characters/Yoll/Meshes/Textures/tex6_6.tex6_6" :NewEnumerator6 "/Game/MyStuff/Characters/Yoll/Meshes/Textures/tex6_7.tex6_7" :NewEnumerator7 "/Game/MyStuff/Characters/Yoll/Meshes/Textures/tex6_8.tex6_8" :NewEnumerator8 "/Game/MyStuff/Characters/Yoll/Meshes/Textures/tex6_9.tex6_9" :NewEnumerator9 "/Game/MyStuff/Characters/Yoll/Meshes/Textures/tex6_10.tex6_10" :NewEnumerator10 "/Game/MyStuff/Characters/Yoll/Meshes/Textures/tex6_11.tex6_11"))
  (bind _returnvalue_2 (Rendering|Material|CreateDynamicMaterialInstance (Variables|Default|GetMesh) 4 (Rendering|Material|GetMaterial (Variables|Default|GetMesh) 4) "None" :!class /Script/Engine.PrimitiveComponent))
  (Rendering|Material|SetTextureParameterValue _returnvalue_2 "gltf_tex_diffuse" _returnvalue)
  (Rendering|Material|SetTextureParameterValue _returnvalue_2 "mtoon_tex_ShadeTexture" _returnvalue))

(fn SetPantie
  (Utilities|IsValid (Variables|Appearance|GetPantieRef)
    (:Is%20Valid
      _)
    (:Is%20Not%20Valid
      (bind _returnvalue (AddComponent|AddSkeletalMeshComponent false))
      (Variables|Appearance|SetPantieRef _returnvalue)))
  (Components|SkinnedMesh|SetLeaderPoseComponent (Variables|Appearance|GetPantieRef) (Variables|Default|GetMesh) false false)
  (Transformation|AttachComponentToComponent (Variables|Appearance|GetPantieRef) (Variables|Default|GetMesh) "None" "SnapToTarget" "SnapToTarget" "SnapToTarget" true)
  (Components|SkeletalMesh|SetSkeletalMeshAsset (Variables|Appearance|GetPantieRef) "/Game/MyStuff/Characters/Yoll/Meshes/Outfits/Pantie/Pantie.Pantie")
  (Utilities|IsValid (Variables|Appearance|GetPantie_Outline_Ref)
    (:Is%20Valid
      _)
    (:Is%20Not%20Valid
      (bind _returnvalue_2 (AddComponent|AddSkeletalMeshComponent false (Math|Transform|MakeTransform "0, 0, 0" "0, 0, 0" "-1.000000,-1.000000,-1.000000")))
      (Variables|Appearance|SetPantie_Outline_Ref _returnvalue_2)))
  (Rendering|SetBoundsScale (Variables|Appearance|GetPantie_Outline_Ref) 1e+01)
  (Components|SkeletalMesh|SetSkeletalMeshAsset (Variables|Appearance|GetPantie_Outline_Ref) "/Game/MyStuff/Characters/Yoll/Meshes/Outfits/Pantie/Pantie.Pantie")
  (Rendering|Material|SetMaterial (Variables|Appearance|GetPantie_Outline_Ref) 0 "/Game/MyStuff/Characters/Yoll/Meshes/Materials/M_Yoll_Crt_Outline.M_Yoll_Crt_Outline")
  (Components|SkinnedMesh|SetLeaderPoseComponent (Variables|Appearance|GetPantie_Outline_Ref) (Variables|Appearance|GetPantieRef) false false)
  (Transformation|AttachComponentToComponent (Variables|Appearance|GetPantie_Outline_Ref) (Variables|Appearance|GetPantieRef) "None" "SnapToTarget" "SnapToTarget" "KeepWorld" true))

(fn SetHorn
  (bind _appearance_settings (Variables|Appearance|GetAppearance_Settings))
  (bind _appearance_settings_2 (Variables|Appearance|GetAppearance_Settings))
  (bind _appearance_settings_3 (Variables|Appearance|GetAppearance_Settings))
  (bind _horn_ (Utilities|Struct|BreakS_Yoll_Appearance_Settings _appearance_settings_2))
  (bind _horn_color (Utilities|Struct|BreakS_Yoll_Appearance_Settings _appearance_settings_3))
  (bind _horn__2 (Utilities|Struct|BreakS_Yoll_Appearance_Settings _appearance_settings))
  (bind _returnvalue (select _horn_ "/Game/MyStuff/Characters/Yoll/Meshes/Materials/M_Yoll_Hair_Outline.M_Yoll_Hair_Outline" "/Game/MyStuff/Materials/M_Translucent.M_Translucent"))
  (Utilities|IsValid (Variables|Appearance|GetHornRef)
    (:Is%20Valid
      _)
    (:Is%20Not%20Valid
      (bind _returnvalue_2 (AddComponent|AddSkeletalMeshComponent false))
      (Variables|Appearance|SetHornRef _returnvalue_2)))
  (Components|SkinnedMesh|SetLeaderPoseComponent (Variables|Appearance|GetHornRef) (Variables|Default|GetMesh) false false)
  (Transformation|AttachComponentToComponent (Variables|Appearance|GetHornRef) (Variables|Default|GetMesh) "None" "SnapToTarget" "SnapToTarget" "SnapToTarget" true)
  (Components|SkeletalMesh|SetSkeletalMeshAsset (Variables|Appearance|GetHornRef) "/Game/MyStuff/Characters/Yoll/Meshes/Outfits/Yoll_Horn.Yoll_Horn")
  (Utilities|IsValid (Variables|Appearance|GetHorn_DM)
    (:Is%20Valid
      _)
    (:Is%20Not%20Valid
      (bind _returnvalue_3 (Rendering|Material|CreateDynamicMaterialInstance (Variables|Appearance|GetHornRef) 1 (Rendering|Material|GetMaterial (Variables|Appearance|GetHornRef) 1) "None" :!class /Script/Engine.PrimitiveComponent))
      (Variables|Appearance|SetHorn_DM _returnvalue_3)))
  (Rendering|Material|SetVectorParameterValue (Variables|Appearance|GetHorn_DM) "mtoon_Color" _horn_color :!class /Script/Engine.MaterialInstanceDynamic)
  (Rendering|Material|SetVectorParameterValue (Variables|Appearance|GetHorn_DM) "mtoon_ShadeColor" (* _horn_color "(R=0.700000,G=0.700000,B=0.700000,A=1.000000)") :!class /Script/Engine.MaterialInstanceDynamic)
  (Rendering|Material|SetMaterial (Variables|Appearance|GetHornRef) 0 (select _horn__2 "/Game/MyStuff/Characters/Yoll/Meshes/Materials/M_Yoll_Crt.M_Yoll_Crt" "/Game/MyStuff/Materials/M_Translucent.M_Translucent"))
  (Rendering|Material|SetMaterial (Variables|Appearance|GetHornRef) 1 (select _horn__2 (Variables|Appearance|GetHorn_DM) "/Game/MyStuff/Materials/M_Translucent.M_Translucent"))
  (Utilities|IsValid (Variables|Appearance|GetHorn_Outline_Ref)
    (:Is%20Valid
      _)
    (:Is%20Not%20Valid
      (bind _returnvalue_4 (AddComponent|AddSkeletalMeshComponent false (Math|Transform|MakeTransform "0, 0, 0" "0, 0, 0" "-1.000000,-1.000000,-1.000000")))
      (Variables|Appearance|SetHorn_Outline_Ref _returnvalue_4)))
  (Rendering|SetBoundsScale (Variables|Appearance|GetHorn_Outline_Ref) 1e+01)
  (Components|SkeletalMesh|SetSkeletalMeshAsset (Variables|Appearance|GetHorn_Outline_Ref) "/Game/MyStuff/Characters/Yoll/Meshes/Outfits/Yoll_Horn.Yoll_Horn")
  (Rendering|Material|SetMaterial (Variables|Appearance|GetHorn_Outline_Ref) 0 _returnvalue)
  (Rendering|Material|SetMaterial (Variables|Appearance|GetHorn_Outline_Ref) 1 _returnvalue)
  (Components|SkinnedMesh|SetLeaderPoseComponent (Variables|Appearance|GetHorn_Outline_Ref) (Variables|Appearance|GetHornRef) false false)
  (Transformation|AttachComponentToComponent (Variables|Appearance|GetHorn_Outline_Ref) (Variables|Appearance|GetHornRef) "None" "SnapToTarget" "SnapToTarget" "KeepWorld" true))

(fn UpdateAppearance
  (InitialSetups|SetHair)
  (InitialSetups|SetCloth)
  (InitialSetups|SetSkin)
  (InitialSetups|SetEye)
  (InitialSetups|SetHorn))

(fn ResetClothMaterial
  (bind _clothref (Variables|Appearance|GetClothRef))
  (for (_array_element _array_index) (Variables|/Script/Engine.SkeletalMesh|GetMaterials (Variables|/Script/Engine.SkeletalMeshComponent|GetSkeletalMeshAsset _clothref))
    (Rendering|Material|SetMaterial _clothref _array_index (.MaterialInterface (Utilities|Struct|BreakSkeletalMaterial _array_element)))))