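; Combat actor component that runs weapon-style socket traces and stamina regeneration on the server, extending parent trace events.
; TraceStart stores a looping, near-per-frame Timer_Trace timer in a map keyed by start socket, replacing any existing one; TraceEnd clears it.
; A looping timer adds stamina at a set rate.
; Any stamina drop pauses regeneration, and a retriggerable delay resumes it after a short period without further loss.
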(event EventBeginPlay
  (Networking|SwitchHasAuthority
    (:Authority
      (|StaminaRegenerate))))

(event EventTick
  (params (DeltaSeconds :type Float%20%28single-precision%29)))

(event EventTraceStart
  (params (TraceInfo :type Trace%20Info%20Structure))
  (bind _start (Utilities|Struct|BreakTraceInfo TraceInfo))
  (bind _traceinfos (Variables|Default|GetTraceInfos))
  (bind (_value _returnvalue) (Utilities|Map|Find _traceinfos _start))
  ;[0.7578 1 0] Trace
  (Networking|SwitchHasAuthority
    (:Authority
      (|CallParentFunction TraceInfo)
      (if _returnvalue
        (Utilities|Time|ClearandInvalidateTimerbyHandle (.TimerHandle (Utilities|Struct|BreakTraceInfo _value))))
      (bind _returnvalue_2 (Utilities|Time|SetTimerbyFunctionName 0 "Timer_Trace" 0.001 true))
      (bind _structout (Utilities|Struct|SetmembersinTraceInfo TraceInfo _returnvalue_2))
      (Utilities|Map|Add (Variables|Default|GetTraceInfos) _start _structout))))

(event EventOnRepTagContainer
  (params (Previous :type Gameplay%20Tag%20Container%20Structure))
  (|CallParentFunction Previous))

(event EventTraceEnd
  (params (SocketName :type Name :default "None"))
  (bind _traceinfos (Variables|Default|GetTraceInfos))
  (bind (_value _returnvalue) (Utilities|Map|Find _traceinfos SocketName))
  ;[0.7578 1 0] Trace
  (Networking|SwitchHasAuthority
    (:Authority
      (|CallParentFunction SocketName)
      (if _returnvalue
        (Utilities|Time|ClearandInvalidateTimerbyHandle (.TimerHandle (Utilities|Struct|BreakTraceInfo _value)))
        (Utilities|Map|Remove _traceinfos SocketName)))))

(event Custom|StaminaRegen
  (Class|CombatComponent|AddStamina (* (Variables|Default|GetStaminaReg_Rate) 0.1)))

(event Custom|StopStaminaReg
  (bind _staminareg_handle (Variables|Default|GetStaminaReg_Handle))
  (Utilities|Time|PauseTimerbyHandle _staminareg_handle)
  (Utilities|FlowControl|RetriggerableDelay 2.0)
  (Utilities|Time|UnpauseTimerbyHandle _staminareg_handle))

(event Custom|OnStaminaChanged
  (params (Before :type Float%20%28single-precision%29) (After :type Float%20%28single-precision%29))
  (if (< After Before)
    (CallFunction|StopStaminaReg)))