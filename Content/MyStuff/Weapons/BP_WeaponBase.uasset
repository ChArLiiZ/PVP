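; Base weapon actor that removes itself from the game when it is no longer its owner's referenced weapon.
; A looping one-second timer started on BeginPlay destroys the actor if the owner's WeaponRef is invalid or points to another object.
; The StopCheck event sets a flag that makes the next timer tick clear the timer, leaving the actor in place.
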(event Custom|CheckOwner
  (if (Variables|Default|GetStopCheck?)
    (Utilities|Time|ClearandInvalidateTimerbyHandle (stale EventBeginPlay _returnvalue) :!label _label)
    (else
      (bind _weaponref (Variables|/Script/PVP.PVPCharacter|GetWeaponRef (Variables|Default|GetOwnerRef))
        (:then
          (if (not (== _weaponref self))
            (Actor|DestroyActor :!label _label_2)
            (goto _label)))
        (:else
          (goto _label_2))))))

(event Custom|StopCheck
  (Variables|Default|SetStopCheck? true))

(event EventBeginPlay
  (bind _returnvalue (Utilities|Time|SetTimerbyEvent (delegate Custom|CheckOwner) 1.0 true)))

(event Collision|EventActorBeginOverlap
  (params (OtherActor :type Actor%20Object%20Reference)))

(event EventTick
  (params (DeltaSeconds :type Float%20%28single-precision%29)))

(fn ConstructionScript)