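; BP_Gaunlet is a paired gauntlet weapon that extends a parent weapon with a second, left-hand piece.
; Setup snaps the Left component to the owner mesh's left gauntlet socket.
; Trail index 1 toggles the left trail, while other indices defer to the parent.
; When a special attack finishes charging, it deducts stamina, draining what remains if that fails, and multicasts a Niagara charge-complete effect.
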(event Custom|OnSpecialAttackChargeCompletedDelegate_Event
  (bind _ownerref (Variables|Default|GetOwnerRef))
  (bind _combatcomponent (Variables|/Script/PVP.PVPCharacter|GetCombatComponent _ownerref))
  (bind _returnvalue (Class|CombatComponent|AddStamina _combatcomponent (* (.SpecialAttackStamina (Utilities|Struct|BreakWeaponAttributes (Variables|/Script/PVP.WeaponInfos|GetAttributes (Variables|Default|GetWeaponInfo)))) -1.0)))
  (if _returnvalue
    _
    (else
      (bind _amount (Class|CombatComponent|GetStamina _combatcomponent false))
      (Class|CombatComponent|AddStamina _combatcomponent (* _amount -1.0))))
  (CallFunction|MulticastChargeComplete))

(event Custom|Multicast_ChargeComplete
  (Niagara|SpawnSystemAttached "/Game/MyStuff/Niagara/NS_ChargeComplete.NS_ChargeComplete" (Variables|Default|GetSKMesh) "None" "0, 0, 0" "0, 0, 0" "KeepRelativeOffset" true true "AutoRelease"))

(event EventBeginPlay
  (|CallParentFunction)
  (EventDispatchers|AssignOnSpecialAttackChargeCompletedDelegate (delegate Custom|OnSpecialAttackChargeCompletedDelegate_Event)))

(event EventInitialSetup
  (|CallParentFunction)
  (Class|WeaponBase|AdditionalSetup (Variables|/Script/Engine.Character|GetMesh (Variables|Default|GetOwnerRef))))

(event EventTrail
  (params (IsStart :type Boolean) (Index :type Integer))
  (bind _trail_l (Variables|Default|GetTrail_L))
  (switch int Index
    (:Default
      (|CallParentFunction IsStart Index))
    (:0
      (|CallParentFunction IsStart Index))
    (:1
      (if IsStart
        (Components|Activation|Activate _trail_l false)
        (else
          (Components|Activation|Deactivate _trail_l))))))

(event EventAdditionalSetup
  (params (SkeletalMesh :type Skeletal%20Mesh%20Component%20Object%20Reference))
  (|CallParentFunction SkeletalMesh)
  (Transformation|AttachComponentToComponent (Variables|Default|GetLeft) SkeletalMesh "Gaunlet_L_Slot" "SnapToTarget" "SnapToTarget" "KeepWorld" true))

(fn ConstructionScript)