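; BP_Halberd is a halberd weapon Blueprint that handles completion of its charged special attack.
; It binds to the charge-completed delegate on BeginPlay, then deducts the special attack's stamina cost through the owner's CombatComponent, draining remaining stamina if that deduction fails.
; A multicast event then spawns an auto-released, pooled Niagara charge-complete effect attached to the skeletal mesh.
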(event Custom|OnSpecialAttackChargeCompletedDelegate_Event
  (bind _ownerref (Variables|Default|GetOwnerRef))
  (bind _combatcomponent (Variables|/Script/PVP.PVPCharacter|GetCombatComponent _ownerref))
  (bind _returnvalue (Class|CombatComponent|AddStamina _combatcomponent (* (.SpecialAttackStamina (Utilities|Struct|BreakWeaponAttributes (Variables|/Script/PVP.WeaponInfos|GetAttributes (Variables|Default|GetWeaponInfo)))) -1.0)))
  (if _returnvalue
    _
    (else
      (bind _amount (Class|CombatComponent|GetStamina _combatcomponent false))
      (Class|CombatComponent|AddStamina _combatcomponent (* _amount -1.0))))
  (CallFunction|MulticastChargeComplete))

(event Custom|Multicast_ChargeComplete
  (Niagara|SpawnSystemAttached "/Game/MyStuff/Niagara/NS_ChargeComplete.NS_ChargeComplete" (Variables|Default|GetSKMesh) "None" "0, 0, 0" "0, 0, 0" "KeepRelativeOffset" true true "AutoRelease"))

(event EventBeginPlay
  (EventDispatchers|AssignOnSpecialAttackChargeCompletedDelegate (delegate Custom|OnSpecialAttackChargeCompletedDelegate_Event)))

(fn ConstructionScript)